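; BP_FDGASPlayerController is the player controller that handles game over and respawn for the GAS-based player character.
; On game over it creates the WBP_Dead widget and adds it to the viewport.
; On respawn it moves the pawn to the first PlayerStart, calls Respawn on the FDGASCharacterPlayer and applies the BPGE_Respawn gameplay effect through its ability system component.
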(event Custom|OnPlayerRespawn
  (bind _returnvalue (Game|Player|GetPlayerPawn 0))
  (bind _outactors (Actor|GetAllActorsOfClass "/Script/Engine.PlayerStart"))
  (Transformation|SetActorLocation _returnvalue (Transformation|GetActorLocation (Utilities|Array|Get(acopy) _outactors)) false false)
  (bind _asfdgascharacter_player (Utilities|Casting|CastToFDGASCharacterPlayer _returnvalue))
  (Class|FDCharacterPlayer|Respawn _asfdgascharacter_player)
  (GameplayEffects|ApplyGameplayEffectToSelf :self (Ability|GetAbilitySystemComponent _asfdgascharacter_player) :GameplayEffectClass "/Game/FDPorjectGAS/Blueprint/GE/BPGE_Respawn.BPGE_Respawn_C"))

(event EventBeginPlay)

(event EventTick
  (params (DeltaSeconds :type Float%20%28single-precision%29)))

(event EventOnGameOver
  (bind _returnvalue (UserInterface|CreateWidget "/Game/FDPorjectGAS/UI/WBP_Dead.WBP_Dead_C"))
  (UserInterface|Viewport|AddtoViewport _returnvalue 0))

(fn ConstructionScript)