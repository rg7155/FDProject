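; GameplayCue notify that shows combo attack animations on characters that are not locally controlled.
; On execute, it casts the target to Character and plays the GAS player combo attack montage, skipping locally controlled instances.
; The cue's rounded raw magnitude serves as the combo index, appended to "ComboAttack" to pick the montage section.
; Debug prints show the chosen section or a failed cast.
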(fn OnExecute
  (params (MyTarget :type Actor%20Object%20Reference) (Parameters :type Gameplay%20Cue%20Parameters%20Structure%20%28by%20ref%29))
  (bind _rawmagnitude (Ability|GameplayCue|BreakGameplayCueParameters Parameters))
  (bind _returnvalue (Math|Float|Round _rawmagnitude))
  (bind _returnvalue_2 (Utilities|String|ToString(Integer) _returnvalue))
  (bind _returnvalue_3 (Utilities|String|Append "ComboAttack" _returnvalue_2))
  (bind _returnvalue_4 (Utilities|String|MakeLiteralString _returnvalue_3))
  (bind _returnvalue_5 (Utilities|String|StringToName _returnvalue_4))
  (bind _ascharacter (Utilities|Casting|CastToCharacter MyTarget)
    (:then
      (if (not (Pawn|IsLocallyControlled _ascharacter))
        (Animation|PlayAnimMontage _ascharacter "/Game/FDPorjectGAS/Animation/AM_GASPlayerComboAttack.AM_GASPlayerComboAttack" 1.0 _returnvalue_5)
        (Development|PrintString 0 (Utilities|String|ToString(Name) _returnvalue_5))))
    (:CastFailed
      (Development|PrintString 0 "failed"))))