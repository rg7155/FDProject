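; Gameplay Cue notify actor that shows the visual effect for an attack rate buff on a character.
; OnActive casts the target to Character, attaches a fire buff particle to the sword_top socket of its mesh and stores the component.
; OnRemove destroys that stored particle component, and both overrides return their parent implementation's result.
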(event EventBeginPlay)

(event Collision|EventActorBeginOverlap
  (params (OtherActor :type Actor%20Object%20Reference)))

(event EventTick
  (params (DeltaSeconds :type Float%20%28single-precision%29)))

(event EventOnReset)

(event GameplayCueNotify|EventHandleGameplayCue
  (params (MyTarget :type Actor%20Object%20Reference) (EventType :type EGameplayCueEvent%20Enum :default "OnActive") (Parameters :type Gameplay%20Cue%20Parameters%20Structure%20%28by%20ref%29)))

(fn ConstructionScript)

(fn OnRemove
  (params (MyTarget :type Actor%20Object%20Reference) (Parameters :type Gameplay%20Cue%20Parameters%20Structure%20%28by%20ref%29))
  (Components|DestroyComponent (Variables|Default|GetParticle))
  (bind _returnvalue (|CallParentFunction MyTarget Parameters))
  (return _returnvalue))

(fn OnActive
  (params (MyTarget :type Actor%20Object%20Reference) (Parameters :type Gameplay%20Cue%20Parameters%20Structure%20%28by%20ref%29))
  (bind _returnvalue (|CallParentFunction MyTarget Parameters))
  (bind _ascharacter (Utilities|Casting|CastToCharacter MyTarget)
    (:then
      (bind _returnvalue_2 (Effects|SpawnEmitterAttached "/Game/InfinityBladeEffects/Effects/FX_Mobile/Fire/combat/P_Buff_JumpDiveFire_01.P_Buff_JumpDiveFire_01" (Variables|/Script/Engine.Character|GetMesh _ascharacter) "sword_top"))
      (Variables|Default|SetParticle _returnvalue_2))
    (:CastFailed
      _))
  (return _returnvalue))